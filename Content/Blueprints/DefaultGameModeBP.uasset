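; Game mode for a two-player local match that spawns both players' chosen characters and links them as opponents or partners.
; On BeginPlay it finds PlayerStarts tagged P1 and P2, spawns the Gideon or Phase character selected in BaseGameInstance, and possesses each with its player controller.
; Once both are valid, each gets a reference to the other and a shared CharacterHUD is created for controller 0.
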(event EventBeginPlay
  (bind _player1 (Variables|Default|Getplayer1))
  (bind _player2 (Variables|Default|Getplayer2))
  (bind _outactors (Actor|GetAllActorsOfClass "/Script/Engine.PlayerStart"))
  (for _array_element _outactors
    (CallFunction|SpawnPlayers _array_element))
  (if (Utilities|IsValid (Variables|Default|Getplayer1))
    (if (Utilities|IsValid (Variables|Default|Getplayer2))
      (Variables|/Script/FighterAssignment.FighterAssignmentCharacter|SetOtherPlayer _player1 _player2)
      (Variables|/Script/FighterAssignment.FighterAssignmentCharacter|SetOtherPlayer _player2 _player1)
      (bind _returnvalue (UserInterface|CreateWidget "/Game/Blueprints/Widgets/CharacterHUD.CharacterHUD_C" (Game|GetPlayerController 0)))
      (UserInterface|Viewport|AddtoViewport _returnvalue 0))))

(fn ConstructionScript)

(fn SpawnPlayers
  (params (Object :type Actor%20Object%20Reference))
  (bind _asplayer_start (Utilities|Casting|CastToPlayerStart Object))
  (if (Utilities|Name|Equal(Name) (Variables|/Script/Engine.PlayerStart|GetPlayerStartTag _asplayer_start) "P1")
    (bind _character_reference (CallFunction|DetermineCharacterClass (Transformation|GetActorTransform Object) Object))
    (Variables|Default|Setplayer1 _character_reference)
    (Pawn|Possess (Game|GetPlayerController 0) _character_reference)
    (elif (Utilities|Name|Equal(Name) (Variables|/Script/Engine.PlayerStart|GetPlayerStartTag _asplayer_start) "P2")
      (bind _character_reference_2 (CallFunction|DetermineCharacterClass (Transformation|GetActorTransform Object) Object 1))
      (Variables|Default|Setplayer2 _character_reference_2)
      (Pawn|Possess (Game|GetPlayerController 1) _character_reference_2))))

(fn DetermineCharacterClass
  (params (Transform :type Transform) (Actor :type Actor%20Object%20Reference) (PlayerIndex :type Integer))
  (bind _asbase_game_instance (Utilities|Casting|CastToBaseGameInstance (Game|GetGameInstance)))
  (switch int PlayerIndex
    (:0
      (switch Utilities|FlowControl|Switch|SwitchonECharacterClass (Variables|/Script/FighterAssignment.BaseGameInstance|GetP1CharacterClass _asbase_game_instance)
        (:VE_Gideon
          _)
        (:VE_Phase
          (bind _returnvalue (Game|SpawnActorfromClass "/Game/CharacterPhase/PhaseCharacterBP.PhaseCharacterBP_C" Transform "Undefined" Actor 0 :!label _label))
          (return _returnvalue))))
    (:1
      (switch Utilities|FlowControl|Switch|SwitchonECharacterClass (Variables|/Script/FighterAssignment.BaseGameInstance|GetP2CharacterClass _asbase_game_instance)
        (:VE_Gideon
          _)
        (:VE_Phase
          (goto _label)))))
  (bind _returnvalue_2 (Game|SpawnActorfromClass "/Game/CharacterGideon/GideonCharacterBP.GideonCharacterBP_C" Transform "Undefined" Actor 0))
  (return _returnvalue_2))