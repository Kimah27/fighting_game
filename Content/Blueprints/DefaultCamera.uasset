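; Shared camera for a two-player fighting game that frames both fighters along the Y axis.
; Each Tick it reads both players and the round state from DefaultGameModeBP.
; During a fight it clamps each player's Y to a band around the camera, then moves to their midpoint at fixed depth, with bounded Y and slightly raised height.
; Outside a fight, it snaps to a fixed start position while a round is starting.
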(event EventTick
  (params (DeltaSeconds :type Float%20%28single-precision%29))
  (bind _returnvalue (Transformation|GetActorLocation))
  (bind _returnvalue_2 (Transformation|GetActorLocation))
  (bind _y (Math|Vector|BreakVector _returnvalue_2))
  (bind _y_2 (Math|Vector|BreakVector _returnvalue))
  (bind _asdefault_game_mode_bp (Utilities|Casting|CastToDefaultGameModeBP (Game|GetGameMode)))
  (Utilities|IsValid (Variables|/Script/FighterAssignment.FighterAssignmentGameMode|Getplayer1 _asdefault_game_mode_bp)
    (:Is%20Valid
      (Variables|Default|SetPlayer1Reference (Variables|/Script/FighterAssignment.FighterAssignmentGameMode|Getplayer1 _asdefault_game_mode_bp))
      (Utilities|IsValid (Variables|/Script/FighterAssignment.FighterAssignmentGameMode|Getplayer2 _asdefault_game_mode_bp)
        (:Is%20Valid
          (Variables|Default|SetPlayer2Reference (Variables|/Script/FighterAssignment.FighterAssignmentGameMode|Getplayer2 _asdefault_game_mode_bp))
          (if (Variables|/Script/FighterAssignment.FighterAssignmentGameMode|GetfightBegun _asdefault_game_mode_bp)
            (Transformation|SetActorLocation (Variables|Default|GetPlayer1Reference) (Math|Vector|MakeVector (.X (Math|Vector|BreakVector (Transformation|GetActorLocation (Variables|Default|GetPlayer1Reference)))) (Math|Float|Clamp(Float) (.Y (Math|Vector|BreakVector (Transformation|GetActorLocation (Variables|Default|GetPlayer1Reference)))) (- _y 3e+02) (+ _y 3e+02)) (.Z (Math|Vector|BreakVector (Transformation|GetActorLocation (Variables|Default|GetPlayer1Reference))))) false false)
            (Transformation|SetActorLocation (Variables|Default|GetPlayer2Reference) (Math|Vector|MakeVector (.X (Math|Vector|BreakVector (Transformation|GetActorLocation (Variables|Default|GetPlayer2Reference)))) (Math|Float|Clamp(Float) (.Y (Math|Vector|BreakVector (Transformation|GetActorLocation (Variables|Default|GetPlayer2Reference)))) (- _y_2 3e+02) (+ _y_2 3e+02)) (.Z (Math|Vector|BreakVector (Transformation|GetActorLocation (Variables|Default|GetPlayer2Reference))))) false false)
            (if (and (Utilities|IsValid (Variables|Default|GetPlayer1Reference)) (Utilities|IsValid (Variables|Default|GetPlayer2Reference)))
              (Transformation|SetActorLocation (Math|Vector|MakeVector (Math|Conversions|ToFloat(Integer) (Math|Float|Round 4e+02)) (/ (Math|Float|Clamp(Float) (+ (.Y (Math|Vector|BreakVector (Transformation|GetActorLocation (Variables|Default|GetPlayer1Reference)))) (.Y (Math|Vector|BreakVector (Transformation|GetActorLocation (Variables|Default|GetPlayer2Reference))))) -1.2e+03 1.2e+03) 2.0) (/ (+ (+ (.Z (Math|Vector|BreakVector (Transformation|GetActorLocation (Variables|Default|GetPlayer1Reference)))) (.Z (Math|Vector|BreakVector (Transformation|GetActorLocation (Variables|Default|GetPlayer2Reference))))) 7e+01) 2.0)) false false))
            (elif (Variables|/Script/FighterAssignment.FighterAssignmentGameMode|GetroundStarting _asdefault_game_mode_bp)
              (Transformation|SetActorLocation "400.000000, 0,133.149994" false false))))))))

(fn ConstructionScript)